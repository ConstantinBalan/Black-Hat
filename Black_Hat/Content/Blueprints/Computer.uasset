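; Computer is an interactable prop actor that highlights and labels itself when the mouse cursor hovers over it.
; Cursor-over events on the static mesh toggle custom depth rendering, typically used for outline effects.
; The same events set ObjectName to "Computer" or clear it, then push it to the ComputerText component.
; The construction script initializes the text from ObjectName.
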(event `self.StaticMeshComponent.OnBeginCursorOver`
  (params (TouchedComponent :type "PrimitiveComponent Object Reference"))
  (`PrimitiveComponent.SetRenderCustomDepth` (`self.StaticMeshComponent`) true)
  (bind _output_get (set `self.ObjectName` "Computer"))
  (`TextRenderComponent.K2_SetText` (`self.Computer Text`) _output_get))

(event `self.StaticMeshComponent.OnEndCursorOver`
  (params (TouchedComponent :type "PrimitiveComponent Object Reference"))
  (`PrimitiveComponent.SetRenderCustomDepth` (`self.StaticMeshComponent`) false)
  (bind _output_get (set `self.ObjectName` ""))
  (`TextRenderComponent.K2_SetText` (`self.Computer Text`) _output_get))

(fn `UserConstructionScript`
  (`TextRenderComponent.K2_SetText` (`self.Computer Text`) (`self.ObjectName`)))